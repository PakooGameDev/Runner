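; LevelManager is an actor that drives the level's background plane behind the player character.
; Every tick it moves the plane to the player's X position at a fixed Y, so the backdrop follows horizontal movement.
; It applies the background material on BeginPlay, then a looping timer polls MainCharacter's IsDead flag and swaps in a static material upon death.
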(event `self.ReceiveTick`
  (params (DeltaSeconds :type "Float (single-precision)"))
  (`self.UpdateBackgroudPosition`))

(event `self.ReceiveBeginPlay`
  (`PrimitiveComponent.SetMaterial` (`self.Plane`) 0 "/Game/Materials/M_Background.M_Background")
  (`KismetSystemLibrary.K2_SetTimerDelegate` (delegate `CheckTheDeath`) 0.1 true))

(event `CheckTheDeath`
  (if (`/Game/Blueprints/MainCharacter.IsDead` (cast `/Game/Blueprints/MainCharacter` (`GameplayStatics.GetPlayerCharacter` 0) :!pure true))
    (`PrimitiveComponent.SetMaterial` (`self.Plane`) 0 "/Game/Materials/M_BackgroundStatic.M_BackgroundStatic")))

(fn `UpdateBackgroudPosition`
  (bind _returnvalue (`GameplayStatics.GetPlayerCharacter` 0))
  (bind _returnvalue_x (`KismetMathLibrary.BreakVector` (`self.K2_GetActorLocation` _returnvalue)))
  (`/Engine/EditorBlueprintResources/StandardMacros.IsValid` _returnvalue
    (:`Is Valid`
      (`SceneComponent.K2_SetWorldLocation` (`self.Plane`) (`KismetMathLibrary.MakeVector` _returnvalue_x -500.0) false false))))

(fn `UserConstructionScript`)