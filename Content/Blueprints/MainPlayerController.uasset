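; MainPlayerController manages an endlessly recycled level of floor tiles.
; On BeginPlay it spawns a row of FloorBase tiles, placing each one a fixed distance along the last tile's forward vector, using only the X coordinate.
; The UpdateLevel event destroys the oldest tile and appends either a FloorBase or a FloorBridge_ at random.
; SpawnObstacle is an empty stub.
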(event `self.ReceiveBeginPlay`
  (bind _returnvalue (`|SpawnActorFromClass` "/Game/Blueprints/Floors/FloorBase.FloorBase_C" (`KismetMathLibrary.MakeTransform` (-6858.0 0.0 0.0)) "Undefined" "OverrideRootScale" null null))
  (`KismetArrayLibrary.Array_Add` (`self.Floors`) _returnvalue)
  (for _ (range 4)
    (bind _returnvalue_2 (`|SpawnActorFromClass` "/Game/Blueprints/Floors/FloorBase.FloorBase_C" (`KismetMathLibrary.MakeTransform` (`KismetMathLibrary.MakeVector` (`self.GetAttachPosition`))) "Undefined" "OverrideRootScale" null null))
    (`KismetArrayLibrary.Array_Add` (`self.Floors`) _returnvalue_2)))

(event `UpdateLevel`
  (`self.UpdateTiles `))

(fn `GetAttachPosition`
  (returns (ReturnValue_X :type "Float (double-precision)"))
  (bind _floors (`self.Floors`))
  (bind _output (`|GetArrayItem` _floors (`KismetArrayLibrary.Array_LastIndex` _floors)))
  (bind _returnvalue_x (`KismetMathLibrary.BreakVector` (+ (* (`self.GetActorForwardVector` _output) 2286.0) (`self.K2_GetActorLocation` _output))))
  (`/Engine/EditorBlueprintResources/StandardMacros.IsValid` _output
    (:`Is Valid`
      (return _returnvalue_x))))

(fn `SpawnObstacle`
  (params (Target :type "Actor Object Reference")))

(fn `UpdateTiles `
  (bind _floors (`self.Floors`))
  (bind _output (`|GetArrayItem` _floors))
  (`/Engine/EditorBlueprintResources/StandardMacros.IsValid` _output
    (:`Is Valid`
      (`self.K2_DestroyActor` _output)
      (bind _returnvalue (`KismetArrayLibrary.Array_RemoveItem` _floors _output))
      (if _returnvalue
        (bind _returnvalue_2 (`|SpawnActorFromClass` (select `int` (`KismetMathLibrary.RandomIntegerInRange` 0 1) :`0` "/Game/Blueprints/Floors/FloorBase.FloorBase_C" :`1` "/Game/Blueprints/Floors/FloorBridge_.FloorBridge__C" :!type "Actor Class Reference") (`KismetMathLibrary.MakeTransform` (`KismetMathLibrary.MakeVector` (`self.GetAttachPosition`))) "Undefined" "OverrideRootScale" null null))
        (`KismetArrayLibrary.Array_Add` (`self.Floors`) _returnvalue_2)))))

(fn `UserConstructionScript`)