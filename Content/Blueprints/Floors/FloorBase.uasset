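; FloorBase is a floor segment that can fill itself with random obstacles and coins at BeginPlay when its SpawnObstacles flag is set.
; It adds child actors at arrow markers: either one wood, stone or coin piece, or several saw or coin pieces at a second arrow set.
; A saw roll can activate the saw sound.
; When MainCharacter leaves the box trigger, MainPlayerController updates the level.
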(event `self.ReceiveBeginPlay`
  (if (`self.SpawnObstacles?`)
    (`self.SpawnObstacles`)))

(event `self.Box.OnComponentEndOverlap`
  (params (OverlappedComponent :type "PrimitiveComponent Object Reference") (OtherActor :type "Actor Object Reference") (OtherComp :type "PrimitiveComponent Object Reference") (OtherBodyIndex :type Integer))
  (bind _asmain_character (cast `/Game/Blueprints/MainCharacter` OtherActor))
  (`/Engine/EditorBlueprintResources/StandardMacros.IsValid` _asmain_character
    (:`Is Valid`
      (bind _asmain_player_controller (cast `/Game/Blueprints/MainPlayerController` (`GameplayStatics.GetPlayerController` 0)))
      (`/Game/Blueprints/MainPlayerController.UpdateLevel` _asmain_player_controller))))

(fn `GetRandomSpawnPoint`
  (params (Index :type Integer))
  (returns (SpawnPoint :type "Vector Structure"))
  (locals (Save :type "Vector Structure"))
  (bind _array (`|MakeArray` (`SceneComponent.RelativeLocation` (`self.Arrow4`)) (`SceneComponent.RelativeLocation` (`self.Arrow5`)) (`SceneComponent.RelativeLocation` (`self.Arrow6`)) (`SceneComponent.RelativeLocation` (`self.Arrow7`))))
  (`KismetArrayLibrary.Array_Shuffle` _array)
  (return (`|GetArrayItem` _array Index)))

(fn `SpawnObstacles`
  (locals (L_SavedObstLoc :type "Vector Structure"))
  (bind _returnvalue (`KismetMathLibrary.RandomIntegerInRange` 0 1))
  (bind _returnvalue_2 (select `int` _returnvalue :`0` "/Game/Blueprints/Obstacles/Saws.Saws_C" :`1` "/Game/Blueprints/Obstacles/Coins.Coins_C" :!type "Actor Class Reference"))
  (switch `int` _returnvalue
    (:`0`
      (bind _returnvalue_3 (`AddComponent|NODE_AddChildActorComponent-0` :`RelativeTransform` (`KismetMathLibrary.MakeTransform` (select `int` (`KismetMathLibrary.RandomIntegerInRange` 0 3) :`0` (`SceneComponent.RelativeLocation` (`self.Arrow`)) :`1` (`SceneComponent.RelativeLocation` (`self.Arrow1`)) :`2` (`SceneComponent.RelativeLocation` (`self.Arrow2`)) :`3` (`SceneComponent.RelativeLocation` (`self.Arrow3`))))))
      (`ChildActorComponent.SetChildActorClass` _returnvalue_3 (select `int` (`KismetMathLibrary.RandomIntegerInRange` 0 2) :`0` "/Game/Blueprints/Obstacles/Woods.Woods_C" :`1` "/Game/Blueprints/Obstacles/Stones.Stones_C" :`2` "/Game/Blueprints/Obstacles/Coins.Coins_C" :!type "Actor Class Reference")))
    (:`1`
      (for _index (range (+ (`KismetMathLibrary.RandomIntegerInRange` 1 3) 1))
        (bind _returnvalue_4 (`AddComponent|NODE_AddChildActorComponent-2` :`RelativeTransform` (`KismetMathLibrary.MakeTransform` (`self.GetRandomSpawnPoint` _index))))
        (if (== _returnvalue_2 "/Game/Blueprints/Obstacles/Saws.Saws_C")
          (`ActorComponent.SetActive` (`self.sawSound_Cue`) true false))
        (`ChildActorComponent.SetChildActorClass` _returnvalue_4 _returnvalue_2)))))

(fn `UserConstructionScript`)